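; AttackNotify is an animation notify state that deals sword damage during attacks.
; Each tick, it casts player pawn 0 to FirstPersonCharacter and sphere-traces between the SwordStart and SwordEnd sockets on its EquippedWeapon, with debug drawing on.
; It applies the weapon's DMG to the hit actor on every tick, without tracking actors already hit.
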(fn `Received_NotifyTick`
  (params (MeshComp :type "SkeletalMeshComponent Object Reference") (Animation :type "AnimSequenceBase Object Reference") (FrameDeltaTime :type "Float (double-precision)"))
  (returns (ReturnValue :type Boolean))
  ;[1 1 1] Creates a Line trace from the start of the sword to the point of the sword, deals damage based on information stored in the equipped weapon
  (bind _asfirst_person_character (cast `/Game/FPSwordAndShield/Blueprints/FirstPersonCharacter` (`GameplayStatics.GetPlayerPawn` MeshComp)))
  (bind _equipped_weapon (`/Game/FPSwordAndShield/Blueprints/FirstPersonCharacter.Equipped Weapon` _asfirst_person_character))
  (bind _outhit (`KismetSystemLibrary.SphereTraceSingle` :`WorldContextObject` MeshComp :`Start` (`SceneComponent.GetSocketLocation` (`Actor.RootComponent` _equipped_weapon) "SwordStart") :`End` (`SceneComponent.GetSocketLocation` (`Actor.RootComponent` _equipped_weapon) "SwordEnd") :`Radius` 3.0 :`TraceChannel` "TraceTypeQuery2" :`bTraceComplex` true :`DrawDebugType` "ForDuration"))
  (`GameplayStatics.ApplyDamage` (`.HitActor` (`GameplayStatics.BreakHitResult` _outhit)) (`KismetMathLibrary.Conv_IntToDouble` (`/Game/FPSwordAndShield/Blueprints/Weapons/BaseWeapon.DMG` _equipped_weapon)))
  (return false))