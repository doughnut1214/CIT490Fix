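; StamPickup is a stamina pickup that refills the first-person player's stamina to full when consumed.
; Its Consume event runs CoolDown, which is defined outside this graph, then calls SetStam.
; SetStam casts player pawn 0 to FirstPersonCharacter and sets CurrentStam to MaxStam, so it always affects that player regardless of what triggered the pickup.
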(event `self.Consume`
  (`self.CoolDown`)
  (`self.setStam`))

(fn `setStam`
  (bind _asfirst_person_character (cast `/Game/FPSwordAndShield/Blueprints/FirstPersonCharacter` (`GameplayStatics.GetPlayerPawn` 0)))
  (set `/Game/FPSwordAndShield/Blueprints/FirstPersonCharacter.CurrentStam` (`/Game/FPSwordAndShield/Blueprints/FirstPersonCharacter.MaxStam` _asfirst_person_character) _asfirst_person_character))

(fn `UserConstructionScript`
  (`parent.UserConstructionScript`))