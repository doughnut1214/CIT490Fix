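; Base pickup Blueprint for health or stamina items, noted as able to spawn in place of purchasable weapons in rooms.
; A rotating mesh fires the Consume event when the first player's pawn overlaps its sphere while available.
; Consume grants nothing here and only calls CoolDown, which hides and disables the pickup until a short timer calls Reactivate to restore it.
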(event `self.ReceiveBeginPlay`
  ;[1 1 1] A simple object that will serve to pickup health or stamina, have a chance to spawn in place of a purchasable weapon in rooms
  (`MovementComponent.SetUpdatedComponent` (`self.RotatingMovement`) (`self.Pickup`)))

(event `self.Sphere.OnComponentBeginOverlap`
  (params (OverlappedComponent :type "PrimitiveComponent Object Reference") (OtherActor :type "Actor Object Reference") (OtherComp :type "PrimitiveComponent Object Reference") (OtherBodyIndex :type Integer) (bFromSweep :type Boolean) (SweepResult :type "HitResult Structure (by ref)"))
  (if (and (== OtherActor (`GameplayStatics.GetPlayerPawn` 0)) (`self.isAvailable`))
    (`self.Consume`)))

(event `Consume`
  (`self.CoolDown`))

(fn `CoolDown`
  (`KismetSystemLibrary.K2_SetTimer` null "Reactivate" 5.0)
  (`SceneComponent.SetVisibility` (`self.Pickup`) false false)
  (set `self.isAvailable` false))

(fn `Reactivate`
  (set `self.isAvailable` true)
  (`SceneComponent.SetVisibility` (`self.Pickup`) true false))

(fn `UserConstructionScript`)