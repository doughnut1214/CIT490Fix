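; BaseWeapon is a base weapon actor that the FirstPersonCharacter can buy with points and pick up.
; Entering its Trigger creates an Activate widget showing the Cost and enables input on the actor; leaving removes the widget and disables input.
; Pressing Activate with enough Points passes the weapon to the character's PickUpWeapon, spends the Cost, removes the prompt and disables input.
; Leftover physics-reset and destroy nodes are unconnected.
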(event `InputAction|Activate`
  (params (Key :type "Key Structure"))
  (:`Pressed`
    (bind _asfirst_person_character (cast `/Game/FPSwordAndShield/Blueprints/FirstPersonCharacter` (`GameplayStatics.GetPlayerPawn` 0)))
    (if (>= (`/Game/FPSwordAndShield/Blueprints/FirstPersonCharacter.Points` _asfirst_person_character) (`self.Cost`))
      (`/Game/FPSwordAndShield/Blueprints/FirstPersonCharacter.PickUpWeapon` _asfirst_person_character self)
      (`self.DisableInput` null)
      (`/Game/FPSwordAndShield/Blueprints/FirstPersonCharacter.SpendPoints` _asfirst_person_character (`self.Cost`))
      (bind _foundwidgets (`WidgetBlueprintLibrary.GetAllWidgetsOfClass` "/Game/FPSwordAndShield/Blueprints/Activate.Activate_C"))
      (`Widget.RemoveFromParent` _foundwidgets)
      (`self.DisableInput` null))))

(event `self.Trigger.OnComponentBeginOverlap`
  (params (OverlappedComponent :type "PrimitiveComponent Object Reference") (OtherActor :type "Actor Object Reference") (OtherComp :type "PrimitiveComponent Object Reference") (OtherBodyIndex :type Integer) (bFromSweep :type Boolean) (SweepResult :type "HitResult Structure (by ref)"))
  (bind _returnvalue (`GameplayStatics.GetPlayerController` 0))
  (cast `/Game/FPSwordAndShield/Blueprints/FirstPersonCharacter` OtherActor)
  (bind _returnvalue_2 (`|CreateWidget` "/Game/FPSwordAndShield/Blueprints/Activate.Activate_C" _returnvalue))
  (`/Game/FPSwordAndShield/Blueprints/Activate.GetCost` _returnvalue_2 (`self.Cost`))
  (`UserWidget.AddToViewport` _returnvalue_2 0)
  (`self.EnableInput` _returnvalue))

(event `self.Trigger.OnComponentEndOverlap`
  (params (OverlappedComponent :type "PrimitiveComponent Object Reference") (OtherActor :type "Actor Object Reference") (OtherComp :type "PrimitiveComponent Object Reference") (OtherBodyIndex :type Integer))
  (cast `/Game/FPSwordAndShield/Blueprints/FirstPersonCharacter` OtherActor)
  (bind _foundwidgets (`WidgetBlueprintLibrary.GetAllWidgetsOfClass` "/Game/FPSwordAndShield/Blueprints/Activate.Activate_C"))
  (`Widget.RemoveFromParent` _foundwidgets)
  (`self.DisableInput` null))

(fn `UserConstructionScript`)